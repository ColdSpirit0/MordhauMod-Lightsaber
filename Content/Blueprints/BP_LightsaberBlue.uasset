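; Blue lightsaber weapon for Mordhau that queues dismemberment on any severable bone it hits.
; On cosmetic clients, the construction script adds the blade mesh and audio component, and BeginPlay picks a random hum.
; Tick polls Equipped, Holstered or Dropped, debug-prints it, and on change drives the blade's animation and toggle sound.
; Equipping reveals the blade after a short, rechecked delay; holstering hides it, while dropping leaves mesh visibility untouched.
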(event `self.ReceiveBeginPlay`
  (`parent.ReceiveBeginPlay`)
  (`/Engine/EditorBlueprintResources/StandardMacros.Can Execute Cosmetic Events`
    (:`True`
      (`self.SetupClient`))))

(event `SetupClient`
  (`|ExecutionSequence`
    (:`then_0`
      (bind _asab_lightsaber (cast `/Lightsaber/Blueprints/AB_Lightsaber` (`SkeletalMeshComponent.GetAnimInstance` (`self.BladeSkMesh`))))
      (set `self.Animation` _asab_lightsaber))
    (:`then_1`
      (`AudioComponent.SetIntParameter` (`self.EnabledStateAudio`) "HumNumber" (`KismetMathLibrary.RandomInteger` 5)))))

(event `self.OnHit`
  (params (Actor :type "Actor Object Reference") (Move :type "EAttackMove Enum" :default "RightStrike") (Bone :type Name) (WorldLocation :type "Vector Structure (by ref)") (Tier :type Byte) (SurfaceType :type Byte))
  (`parent.OnHit` Actor Move Bone WorldLocation Tier SurfaceType)
  (bind _asmordhau_character (cast `MordhauCharacter` Actor))
  (if (`MordhauCharacter.CanDismember` _asmordhau_character Bone)
    (`MordhauCharacter.QueueDismember` _asmordhau_character Bone false false (0.0 0.0 0.0) null)))

(event `self.ReceiveTick`
  (params (DeltaSeconds :type "Float (single-precision)"))
  (`parent.ReceiveTick` DeltaSeconds)
  (`/Engine/EditorBlueprintResources/StandardMacros.Can Execute Cosmetic Events`
    (:`True`
      (bind _state (`self.Get Weapon State`))
      (bind _output_get (set `self.LightsaberState` _state))
      (`KismetSystemLibrary.PrintString` (`|GetEnumeratorNameAsString` _output_get) true false (struct :`G` 1.0 :`B` 0.101112 :`A` 1.0) 0.0)
      ;[1 1 1] Check is state changed
      (if (`|EnumInequality` (`self.LightsaberState`) (`self.PreviousState`))
        ;[1 1 1] Update prev state on change
        (set `self.PreviousState` (`self.LightsaberState`))
        (`self.OnClientLightsaberStateUpdated`)))))

(event `OnClientLightsaberStateUpdated`
  (switch `/Lightsaber/Util/ELightsaberState` (`self.LightsaberState`)
    (:`NewEnumerator4`
      ;[1 1 1] Update sound state
      (set `/Lightsaber/Blueprints/AB_Lightsaber.EquipState` (`self.LightsaberState`) (`self.Animation`) :!label _label)
      (if (`self.IsVisuallyEnabled`)
        (`self.Play Toggle Sound` false)
        (else
          (`AudioComponent.SetPaused` (`self.EnabledStateAudio`) true)))
      (set `self.IsVisuallyEnabled` false))
    (:`NewEnumerator3`
      (`SceneComponent.SetVisibility` (`self.BladeSkMesh`) false true)
      (goto _label))
    (:`NewEnumerator2`
      ;[1 1 1] Wait until it get equipped
      (`KismetSystemLibrary.Delay` 0.4)
      ;[1 1 1] is still equipped? (can be dropped while timer ticking)
      (if (`|EnumEquality` (`self.LightsaberState`) "NewEnumerator2")
        (set `self.IsVisuallyEnabled` true)
        ;[1 1 1] Update sound state
        (set `/Lightsaber/Blueprints/AB_Lightsaber.EquipState` (`self.LightsaberState`) (`self.Animation`))
        ;[1 1 1] Play sound
        (`self.Play Toggle Sound` true)
        (`SceneComponent.SetVisibility` (`self.BladeSkMesh`) true true)))))

(event `self.OnEquipped`
  (params (Character :type "MordhauCharacter Object Reference"))
  (`parent.OnEquipped` Character))

(event `self.OnHolstered`
  (params (Character :type "MordhauCharacter Object Reference"))
  (`parent.OnHolstered` Character))

(event `self.OnDropped`
  (params (Character :type "MordhauCharacter Object Reference"))
  (`parent.OnDropped` Character))

(fn `Get Weapon State`
  (returns (State :type "/Lightsaber/Util/ELightsaberState Enum"))
  (if (`self.bIsHeldInHand`)
    (return "NewEnumerator2")
    (elif (`self.BelongsToCharacter`)
      (return "NewEnumerator3")
      (else
        (return "NewEnumerator4")))))

(fn `Play Toggle Sound`
  (params (IsEnabling :type Boolean))
  (`AudioComponent.SetBoolParameter` (`self.EnabledStateAudio`) "Enabled" (`local.IsEnabling`))
  (`AudioComponent.Play` (`self.EnabledStateAudio`) 0.0)
  (`AudioComponent.SetPaused` (`self.EnabledStateAudio`) false))

(fn `UserConstructionScript`
  (`parent.UserConstructionScript`)
  (`/Engine/EditorBlueprintResources/StandardMacros.Can Execute Cosmetic Events`
    (:`True`
      (bind _returnvalue (`AddComponent|NODE_AddSkeletalMeshComponent-0`))
      (set `self.BladeSkMesh` _returnvalue)
      (`/Engine/EditorBlueprintResources/StandardMacros.IsValid` (`self.SaberMaterial`)
        (:`Is Valid`
          (`PrimitiveComponent.SetMaterial` (`self.BladeSkMesh`) 0 (`self.SaberMaterial`)))
        (:`Is Not Valid`
          _))
      (bind _returnvalue_2 (`AddComponent|NODE_AddAudioComponent-0`))
      (set `self.EnabledStateAudio` _returnvalue_2))))